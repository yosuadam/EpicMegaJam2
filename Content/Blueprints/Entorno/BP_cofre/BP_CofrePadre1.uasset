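; Parent chest Blueprint whose lid opens when an overlapping BP_Hada performs its action, optionally requiring a found key (NecesitaLlave).
; Box overlap events store or clear the Hada reference, which Tick polls for LlaveEncontrada and Accionando.
; The Abriendo timeline pitches Tapa open, clearing the key flag during updates if one is required, then spawns BP_Vida at the Arrow on finish.
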(event OnComponentBeginOverlap(Box)
  (params (OverlappedComponent :type Primitive%20Component%20Object%20Reference) (OtherActor :type Actor%20Object%20Reference) (OtherComp :type Primitive%20Component%20Object%20Reference) (OtherBodyIndex :type Integer) (bFromSweep :type Boolean) (SweepResult :type Hit%20Result%20Structure%20%28by%20ref%29))
  (bind _asbp_hada (Utilities|Casting|CastToBP_Hada OtherActor))
  (Variables|Default|SetHada _asbp_hada))

(event OnComponentEndOverlap(Box)
  (params (OverlappedComponent :type Primitive%20Component%20Object%20Reference) (OtherActor :type Actor%20Object%20Reference) (OtherComp :type Primitive%20Component%20Object%20Reference) (OtherBodyIndex :type Integer))
  (Utilities|Casting|CastToBP_Hada OtherActor)
  (Variables|Default|SetHada 0))

(event EventBeginPlay)

(event Collision|EventActorBeginOverlap
  (params (OtherActor :type Actor%20Object%20Reference)))

(event EventTick
  (params (DeltaSeconds :type Float%20%28single-precision%29))
  (bind _necesitallave (Variables|Default|GetnecesitaLlave))
  (bind _hada (Variables|Default|GetHada))
  (bind _hada_2 (Variables|Default|GetHada))
  (Utilities|IsValid _hada
    (:Is%20Valid
      (if _necesitallave
        (if (and _necesitallave (Variables|/Game/Blueprints/Hada/BP_Hada.BP_Hada_C|GetLlaveEncontrada (Variables|Default|GetHada)))
          (if (Variables|/Game/Blueprints/Hada/BP_Hada.BP_Hada_C|GetAccionando? _hada) :!label _label
            (bind _lidfloat (Timeline|Abriendo Play)
              (:Update
                (Transformation|SetRelativeRotation (Variables|Default|GetTapa) (Math|Rotator|MakeRotator 0.0 _lidfloat 0.0) false false)
                (if (Variables|Default|GetnecesitaLlave)
                  (Utilities|IsValid _hada_2
                    (:Is%20Valid
                      (Variables|/Game/Blueprints/Hada/BP_Hada.BP_Hada_C|SetLlaveEncontrada _hada_2 false)))))
              (:Finished
                (Game|SpawnActorfromClass "/Game/Blueprints/Objetos/BP_Vida.BP_Vida_C" (Transformation|GetWorldTransform (Variables|Default|GetArrow)) "Undefined" 0 0)))))
        (else
          (goto _label))))))

(fn ConstructionScript)