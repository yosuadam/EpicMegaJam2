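; Square area-effect Blueprint that reacts to BP_Hada actors entering and leaving its Box, apparently a base for child effects.
; Entry stores the Hada, calls AlEntrar and starts a looping timer targeting MientrasDentro by name, although that function takes a Hada parameter.
; Exit clears the reference, calls AlSalir and stops the timer after a configurable delay.
; All three hook functions are empty here.
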(event OnComponentBeginOverlap(Box)
  (params (OverlappedComponent :type Primitive%20Component%20Object%20Reference) (OtherActor :type Actor%20Object%20Reference) (OtherComp :type Primitive%20Component%20Object%20Reference) (OtherBodyIndex :type Integer) (bFromSweep :type Boolean) (SweepResult :type Hit%20Result%20Structure%20%28by%20ref%29))
  (bind _asbp_hada (Utilities|Casting|CastToBP_Hada OtherActor))
  (bind _output_get (Variables|Default|SetNewVar_0 _asbp_hada))
  (CallFunction|AlEntrar _output_get)
  (bind _returnvalue (Utilities|Time|SetTimerbyFunctionName 0 "MientrasDentro" (Variables|Default|GettimeTick) true)))

(event OnComponentEndOverlap(Box)
  (params (OverlappedComponent :type Primitive%20Component%20Object%20Reference) (OtherActor :type Actor%20Object%20Reference) (OtherComp :type Primitive%20Component%20Object%20Reference) (OtherBodyIndex :type Integer))
  (bind _asbp_hada (Utilities|Casting|CastToBP_Hada OtherActor))
  (Variables|Default|SetNewVar_0 0)
  (CallFunction|AlSalir _asbp_hada)
  (Utilities|FlowControl|Delay (Variables|Default|GettimeDelay))
  (Utilities|Time|ClearandInvalidateTimerbyHandle (stale OnComponentBeginOverlap(Box) _returnvalue)))

(event EventBeginPlay)

(event Collision|EventActorBeginOverlap
  (params (OtherActor :type Actor%20Object%20Reference)))

(event EventTick
  (params (DeltaSeconds :type Float%20%28single-precision%29)))

(fn ConstructionScript)

(fn AlEntrar
  (params (hada :type BP%20Hada%20Object%20Reference)))

(fn AlSalir
  (params (Hada :type BP%20Hada%20Object%20Reference)))

(fn MientrasDentro
  (params (Hada :type BP%20Hada%20Object%20Reference)))