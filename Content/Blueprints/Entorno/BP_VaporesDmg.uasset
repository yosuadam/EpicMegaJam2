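; BP_VaporesDmg is an environmental vapor hazard that damages the fairy (Hada) inside it.
; AlEntrar and MientrasDentro share one path that subtracts a point from SaludActual and prints the result, using the Hada reference supplied by AlEntrar.
; AlSalir only prints an exit message.
; The construction script calls its parent, then sets TimeDelay, which this graph never reads.
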(event EventBeginPlay
  (|CallParentFunction) ; This node is disabled and will not be called.\nDrag off pins to build functionality.
)

(event Collision|EventActorBeginOverlap
  (params (OtherActor :type Actor%20Object%20Reference))
  (|CallParentFunction OtherActor) ; This node is disabled and will not be called.\nDrag off pins to build functionality.
)

(event EventTick
  (params (DeltaSeconds :type Float%20%28single-precision%29))
  (|CallParentFunction DeltaSeconds) ; This node is disabled and will not be called.\nDrag off pins to build functionality.
)

(event EventAlEntrar
  (params (Hada :type BP%20Hada%20Object%20Reference))
  (bind _output_get (Variables|/Game/Blueprints/Hada/BP_Hada.BP_Hada_C|SetSaludActual Hada (- (Variables|/Game/Blueprints/Hada/BP_Hada.BP_Hada_C|GetSaludActual Hada) 1.0)))
  (Development|PrintString (Utilities|String|ToString(Float) _output_get)))

(event EventAlSalir
  (params (Hada :type BP%20Hada%20Object%20Reference))
  (Development|PrintString "As salido"))

(event EventMientrasDentro
  (bind _output_get (Variables|/Game/Blueprints/Hada/BP_Hada.BP_Hada_C|SetSaludActual (stale EventAlEntrar Hada) (- (Variables|/Game/Blueprints/Hada/BP_Hada.BP_Hada_C|GetSaludActual (stale EventAlEntrar Hada)) 1.0)))
  (Development|PrintString (Utilities|String|ToString(Float) _output_get)))

(fn ConstructionScript
  (|CallParentFunction)
  (Variables|Default|SettimeDelay 3e+01))