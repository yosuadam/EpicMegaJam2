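; BP_ZonaMortal is a death zone that drains all health from a fairy (Hada) that enters it.
; Its AlEntrar event sets the fairy's SaludActual to zero and prints the new value to screen.
; The graph has no active overlap, BeginPlay or Tick logic, so detection and the call to AlEntrar come from outside this graph.
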(event EventBeginPlay
  (|CallParentFunction) ; This node is disabled and will not be called.\nDrag off pins to build functionality.
)

(event Collision|EventActorBeginOverlap
  (params (OtherActor :type Actor%20Object%20Reference))
  (|CallParentFunction OtherActor) ; This node is disabled and will not be called.\nDrag off pins to build functionality.
)

(event EventAlEntrar
  (params (hada :type BP%20Hada%20Object%20Reference))
  (bind _output_get (Variables|/Game/Blueprints/Hada/BP_Hada.BP_Hada_C|SetSaludActual hada 0.0))
  (Development|PrintString (Utilities|String|ToString(Float) _output_get)))

(event EventTick
  (params (DeltaSeconds :type Float%20%28single-precision%29))
  (|CallParentFunction DeltaSeconds) ; This node is disabled and will not be called.\nDrag off pins to build functionality.
)

(fn ConstructionScript
  (|CallParentFunction))