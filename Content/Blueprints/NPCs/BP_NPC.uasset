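; Interactable NPC that opens a dialogue when the BP_Hada character performs its action inside the NPC's box trigger.
; Box overlaps store or clear the character reference and toggle a throttled Tick, so polling runs only while it is in range.
; When Tick sees Accionando, it disables movement, replaces all widgets with W_DialogoNPC fed by NPCDialogo, and switches to UI-only input with a visible cursor.
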(event OnComponentEndOverlap(Box)
  (params (OverlappedComponent :type Primitive%20Component%20Object%20Reference) (OtherActor :type Actor%20Object%20Reference) (OtherComp :type Primitive%20Component%20Object%20Reference) (OtherBodyIndex :type Integer))
  ;[1 1 1] Eliminamos la referencia del hada al salir del boxcollision
  (Utilities|Casting|CastToBP_Hada OtherActor)
  (Variables|Default|SetRef_Hada 0)
  (Actor|Tick|SetActorTickEnabled false))

(event OnComponentBeginOverlap(Box)
  (params (OverlappedComponent :type Primitive%20Component%20Object%20Reference) (OtherActor :type Actor%20Object%20Reference) (OtherComp :type Primitive%20Component%20Object%20Reference) (OtherBodyIndex :type Integer) (bFromSweep :type Boolean) (SweepResult :type Hit%20Result%20Structure%20%28by%20ref%29))
  ;[1 1 1] Guardamos una referencia del personaje cuando entra al boxcollision
  (bind _asbp_hada (Utilities|Casting|CastToBP_Hada OtherActor))
  (Variables|Default|SetRef_Hada _asbp_hada)
  (Actor|Tick|SetActorTickEnabled true))

(event EventTick
  (params (DeltaSeconds :type Float%20%28single-precision%29))
  (bind _returnvalue (Game|GetPlayerController 0))
  (bind _ref_hada (Variables|Default|GetRef_Hada))
  ;[1 1 1] Cargamos el widget del diálogo y desactivamos movimiento del pj
  (Utilities|IsValid _ref_hada
    (:Is%20Valid
      (if (Variables|/Game/Blueprints/Hada/BP_Hada.BP_Hada_C|GetAccionando? _ref_hada)
        (Pawn|Components|CharacterMovement|DisableMovement (Variables|/Script/Engine.Character|GetCharacterMovement _ref_hada))
        (Viewport|RemoveAllWidgets)
        (bind _returnvalue_2 (UserInterface|CreateWidget "/Game/Widgets/W_DialogoNPC.W_DialogoNPC_C"))
        (Variables|/Game/Widgets/W_DialogoNPC.W_DialogoNPC_C|SetRefNPC _returnvalue_2 (Variables|DetallesPersonaje|GetNPCDialogo))
        (UserInterface|Viewport|AddtoViewport _returnvalue_2 0)
        (Input|SetInputModeUIOnly _returnvalue _returnvalue_2 "DoNotLock")
        (Variables|/Script/Engine.PlayerController|SetbShowMouseCursor _returnvalue true)))))

(event EventBeginPlay
  ;[1 1 1] Desactivar el evento tick al comenzar el juego y ajustar su intervalo
  (Actor|Tick|SetActorTickEnabled false)
  (Actor|Tick|SetActorTickInterval 0.1))

(fn ConstructionScript)