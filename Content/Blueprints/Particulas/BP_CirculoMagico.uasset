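; BP_CirculoMagico is a short-lived magic circle particle effect actor that fades through a timeline and then removes itself.
; On BeginPlay it creates dynamic material instances for the circle, ring and dot elements of its particle system, then runs the Magia event.
; Magia plays a timeline that drives the shared Visibilidad scalar on all three materials and destroys the actor when the timeline finishes.
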(event Custom|Magia
  (bind _newtrack_0 (Timeline|Timeline_0 Play)
    (:Update
      (Rendering|Material|SetScalarParameterValue (Variables|Default|GetRef_CirculoMagico) "Visibilidad" _newtrack_0 :!class /Script/Engine.MaterialInstanceDynamic))
    (:Finished
      (Actor|DestroyActor))))

(event EventBeginPlay
  (bind _particlesystem (Variables|Default|GetParticleSystem))
  (bind _returnvalue (Rendering|Material|CreateDynamicMaterialInstance _particlesystem 0 "/Game/Materiales/M_CirculoMagico.M_CirculoMagico" :!class /Script/Engine.PrimitiveComponent))
  (Variables|Default|SetRef_CirculoMagico _returnvalue)
  (bind _returnvalue_2 (Rendering|Material|CreateDynamicMaterialInstance _particlesystem 1 "/Game/Materiales/M_AnilloMagico.M_AnilloMagico" :!class /Script/Engine.PrimitiveComponent))
  (Variables|Default|SetRef_AnilloMagico _returnvalue_2)
  (bind _returnvalue_3 (Rendering|Material|CreateDynamicMaterialInstance _particlesystem 2 "/Game/Materiales/M_MagicDot.M_MagicDot" :!class /Script/Engine.PrimitiveComponent))
  (Variables|Default|SetRef_MagicDot _returnvalue_3)
  (CallFunction|Magia))

(fn ConstructionScript)