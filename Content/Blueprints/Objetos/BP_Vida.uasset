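; BP_Vida is a health pickup that heals the BP_Hada character that touches it.
; On Sphere overlap it casts the other actor to BP_Hada, plays the Moneda1 sound at its own location, adds VidaSanada to SaludActual, then destroys itself.
; It also sets LlaveEncontrada (key found) on the character, and the health addition has no clamp here.
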(event OnComponentBeginOverlap(Sphere)
  (params (OverlappedComponent :type Primitive%20Component%20Object%20Reference) (OtherActor :type Actor%20Object%20Reference) (OtherComp :type Primitive%20Component%20Object%20Reference) (OtherBodyIndex :type Integer) (bFromSweep :type Boolean) (SweepResult :type Hit%20Result%20Structure%20%28by%20ref%29))
  (bind _asbp_hada (Utilities|Casting|CastToBP_Hada OtherActor))
  (bind _output_get (Variables|Default|SetHada _asbp_hada))
  (Variables|/Game/Blueprints/Hada/BP_Hada.BP_Hada_C|SetLlaveEncontrada _output_get true)
  (Audio|SpawnSoundatLocation "/Game/Sonidos/Sonidos/moneda1.moneda1" (Transformation|GetWorldLocation (Variables|Default|GetDefaultSceneRoot)))
  (Variables|/Game/Blueprints/Hada/BP_Hada.BP_Hada_C|SetSaludActual (Variables|Default|GetHada) (+ (Math|Conversions|ToFloat(Integer) (Variables|Default|GetVidaSanada)) (Variables|/Game/Blueprints/Hada/BP_Hada.BP_Hada_C|GetSaludActual (Variables|Default|GetHada))))
  (Actor|DestroyActor))

(fn ConstructionScript)